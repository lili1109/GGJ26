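; BP_Cam is a shared two-player camera that takes over the first controller's view and adds a screen-border widget.
; Each tick it projects both players to screen space and grades each axis into edge bands, measuring both axes against viewport width.
; SolveCase chooses zoom out when both hit push bands, move toward a lone pusher, hold in zoom bands, otherwise zoom in.
; UpdatePosition steps spring-arm length within limits or shifts the root.
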(event `self.ReceiveBeginPlay`
  (`PlayerController.SetViewTargetWithBlend` (`GameplayStatics.GetPlayerController` 0) self 0.0 "VTBlend_Linear" 0.0 false)
  (bind _returnvalue (`|CreateWidget` "/Game/Players/Widget/BPW_ScreenBorder.BPW_ScreenBorder_C"))
  (bind _output_get (set `self.WBScreenBorder` _returnvalue))
  (`UserWidget.AddToViewport` _output_get 0)
  (set `SpringArmComponent.bEnableCameraLag` true (`self.SpringArm`))
  (bind _outactors (`GameplayStatics.GetAllActorsOfClass` "/Game/Players/BP_PlayerBase.BP_PlayerBase_C"))
  (set `self.Players` _outactors))

(event `self.ReceiveTick`
  (params (DeltaSeconds :type "Float (single-precision)"))
  (`self.DebugData`)
  (`self.UpdatePosition`))

(fn `AssignAboveBorne`
  (params (PlayerLoc :type "Float (double-precision)") (PushVal :type "Float (double-precision)") (ZoomVal :type "Float (double-precision)") (PlayerBorne :type "/Game/Players/Struct_Enum/STR_PlayerBornes Structure (by ref)") (Xaxis :type "Boolean (by ref)"))
  (locals (DirectionSup :type "/Game/Players/Struct_Enum/EN_Push Enum") (DirectionInf :type "/Game/Players/Struct_Enum/EN_Push Enum"))
  (bind _returnvalue_x (`KismetMathLibrary.BreakVector2D` (`WidgetLayoutLibrary.GetViewportSize`)))
  (`|ExecutionSequence`
    (:`then_0`
      (if Xaxis
        (set `local.DirectionSup` "NewEnumerator3")
        (set `local.DirectionInf` "NewEnumerator2")
        (else
          (set `local.DirectionSup` "NewEnumerator0")
          (set `local.DirectionInf` "NewEnumerator1"))))
    (:`then_1`
      (if (> PlayerLoc (- _returnvalue_x PushVal))
        (`|VariableSetRef` PlayerBorne (make `/Game/Players/Struct_Enum/STR_PlayerBornes` "NewEnumerator2" (`local.DirectionSup`)))
        (elif (> PlayerLoc (- _returnvalue_x ZoomVal))
          (`|VariableSetRef` PlayerBorne (make `/Game/Players/Struct_Enum/STR_PlayerBornes` "NewEnumerator1" (`local.DirectionSup`)))
          (elif (> PlayerLoc ZoomVal)
            (`|VariableSetRef` PlayerBorne (make `/Game/Players/Struct_Enum/STR_PlayerBornes` "NewEnumerator0" "NewEnumerator4"))
            (elif (> PlayerLoc PushVal)
              (`|VariableSetRef` PlayerBorne (make `/Game/Players/Struct_Enum/STR_PlayerBornes` "NewEnumerator1" (`local.DirectionInf`)))
              (else
                (`|VariableSetRef` PlayerBorne (make `/Game/Players/Struct_Enum/STR_PlayerBornes` "NewEnumerator2" (`local.DirectionInf`)))))))))))

(fn `BrusheSelect`
  (params (Borne :type "/Game/Players/Struct_Enum/EN_BornesSelect Enum" :default "NewEnumerator0") (Image :type "Image Object Reference"))
  (returns (`Return Value` :type "/Game/Players/Struct_Enum/STR_Brushes Structure"))
  (switch `/Game/Players/Struct_Enum/EN_BornesSelect` Borne
    (:`NewEnumerator0`
      (return (make `/Game/Players/Struct_Enum/STR_Brushes` (struct :`R` 1.0 :`A` 1.0) Image)))
    (:`NewEnumerator1`
      (return (make `/Game/Players/Struct_Enum/STR_Brushes` (struct :`G` 1.0 :`A` 1.0) Image)))))

(fn `CalcPlayerScreenPos`
  (bind _players (`self.Players`))
  (bind _output (`|GetArrayItem` _players 1))
  (bind _output_2 (`|GetArrayItem` _players))
  (`/Engine/EditorBlueprintResources/StandardMacros.IsValid` _output_2
    (:`Is Valid`
      (`/Engine/EditorBlueprintResources/StandardMacros.IsValid` _output
        (:`Is Valid`
          (set `self.Player1Loc` (`GameplayStatics.ProjectWorldToScreen` null (`self.K2_GetActorLocation` _output_2)))
          (set `self.Player2Loc` (`GameplayStatics.ProjectWorldToScreen` null (`self.K2_GetActorLocation` _output)))
          (return))))))

(fn `CaseSwitching`
  (bind (_player2loc_x _player2loc_y) (`KismetMathLibrary.BreakVector2D` (`self.Player2Loc`)))
  (bind _player2loc_x_2 (`KismetMathLibrary.BreakVector2D` (`self.Player2Loc`)))
  (bind _player1loc_x (`KismetMathLibrary.BreakVector2D` (`self.Player1Loc`)))
  (bind (_zoomdist_x _zoomdist_y) (`KismetMathLibrary.BreakVector2D` (`self.ZoomDist`)))
  (bind _zoomdist_x_2 (`KismetMathLibrary.BreakVector2D` (`self.ZoomDist`)))
  (bind (_pushdist_x _pushdist_y) (`KismetMathLibrary.BreakVector2D` (`self.PushDist`)))
  (bind _pushdist_x_2 (`KismetMathLibrary.BreakVector2D` (`self.PushDist`)))
  (bind (_pushdist_x_3 _pushdist_y_2) (`KismetMathLibrary.BreakVector2D` (`self.PushDist`)))
  (bind _pushdist_x_4 (`KismetMathLibrary.BreakVector2D` (`self.PushDist`)))
  (bind _zoomdist_x_3 (`KismetMathLibrary.BreakVector2D` (`self.ZoomDist`)))
  (bind (_zoomdist_x_4 _zoomdist_y_2) (`KismetMathLibrary.BreakVector2D` (`self.ZoomDist`)))
  (bind (_player1loc_x_2 _player1loc_y) (`KismetMathLibrary.BreakVector2D` (`self.Player1Loc`)))
  (`|ExecutionSequence`
    (:`then_0`
      ;[0.03152 0.03136 0.15 0.5] Player 1
      ;; X
      (`self.AssignAboveBorne` _player1loc_x _pushdist_x_2 _zoomdist_x_2 (`self.Player1BorneX`) true)
      ;; Y
      (`self.AssignAboveBorne` _player1loc_y _pushdist_y _zoomdist_y (`self.Player1BorneY`)))
    (:`then_1`
      ;[0.15 0.007044 0.01342 0.5] Player 2
      ;; X
      (`self.AssignAboveBorne` _player2loc_x_2 _pushdist_x_4 _zoomdist_x_3 (`self.Player2BorneX`) true)
      ;; Y
      (`self.AssignAboveBorne` _player2loc_y _pushdist_y_2 _zoomdist_y_2 (`self.Player2BorneY`)))
    (:`then_2`
      (`self.SolveCase`))))

(fn `DebugData`
  (`self.CalcPlayerScreenPos`)
  (`self.CaseSwitching`))

(fn `IsBorneChanged`
  (params (Color :type "/Game/Players/Struct_Enum/EN_BornesSelect Enum (by ref)") (NextColor :type "/Game/Players/Struct_Enum/EN_BornesSelect Enum" :default "NewEnumerator0") (IsRight :type Boolean))
  (returns (AsChanged :type Boolean))
  (if (`|EnumInequality` Color NextColor)
    (if IsRight
      (set `self.BorneChanged` "NewEnumerator1")
      (`|VariableSetRef` Color NextColor)
      (else
        (set `self.BorneChanged` "NewEnumerator3")
        (`|VariableSetRef` Color NextColor)))
    (return true)
    (else
      (set `self.BorneChanged` "NewEnumerator0")
      (return false))))

(fn `SolveCase`
  (bind _player1bornex_color (break `/Game/Players/Struct_Enum/STR_PlayerBornes` (`self.Player1BorneX`)))
  (bind _player1borney_color (break `/Game/Players/Struct_Enum/STR_PlayerBornes` (`self.Player1BorneY`)))
  (bind _player2bornex_color (break `/Game/Players/Struct_Enum/STR_PlayerBornes` (`self.Player2BorneX`)))
  (bind _player2borney_color (break `/Game/Players/Struct_Enum/STR_PlayerBornes` (`self.Player2BorneY`)))
  (bind _player1bornex_color_2 (break `/Game/Players/Struct_Enum/STR_PlayerBornes` (`self.Player1BorneX`)))
  (bind _player1borney_color_2 (break `/Game/Players/Struct_Enum/STR_PlayerBornes` (`self.Player1BorneY`)))
  (bind _player2bornex_color_2 (break `/Game/Players/Struct_Enum/STR_PlayerBornes` (`self.Player2BorneX`)))
  (bind _player2borney_color_2 (break `/Game/Players/Struct_Enum/STR_PlayerBornes` (`self.Player2BorneY`)))
  (bind (_player1bornex_color_3 _player1bornex_direction) (break `/Game/Players/Struct_Enum/STR_PlayerBornes` (`self.Player1BorneX`)))
  (bind (_player1borney_color_3 _player1borney_direction) (break `/Game/Players/Struct_Enum/STR_PlayerBornes` (`self.Player1BorneY`)))
  (bind (_player2bornex_color_3 _player2bornex_direction) (break `/Game/Players/Struct_Enum/STR_PlayerBornes` (`self.Player2BorneX`)))
  (bind (_player2borney_color_3 _player2borney_direction) (break `/Game/Players/Struct_Enum/STR_PlayerBornes` (`self.Player2BorneY`)))
  (bind _returnvalue (or (`|EnumEquality` _player2bornex_color_2 "NewEnumerator2") (`|EnumEquality` _player2borney_color_2 "NewEnumerator2")))
  (if (or (`|EnumEquality` _player1bornex_color_2 "NewEnumerator2") (`|EnumEquality` _player1borney_color_2 "NewEnumerator2"))
    (if _returnvalue
      (set `self.Direction` (make `/Game/Players/Struct_Enum/STR_Direction2D` "NewEnumerator4" "NewEnumerator4"))
      (set `self.FinaleUpdate` "NewEnumerator1")
      (else
        (set `self.Direction` (make `/Game/Players/Struct_Enum/STR_Direction2D` _player1bornex_direction _player1borney_direction))
        (set `self.FinaleUpdate` "NewEnumerator2")))
    (elif _returnvalue
      (set `self.Direction` (make `/Game/Players/Struct_Enum/STR_Direction2D` _player2bornex_direction _player2borney_direction))
      (set `self.FinaleUpdate` "NewEnumerator2")
      (elif (or (`|EnumEquality` _player1bornex_color "NewEnumerator1") (`|EnumEquality` _player1borney_color "NewEnumerator1") (`|EnumEquality` _player2bornex_color "NewEnumerator1") (`|EnumEquality` _player2borney_color "NewEnumerator1"))
        (set `self.Direction` (make `/Game/Players/Struct_Enum/STR_Direction2D` "NewEnumerator4" "NewEnumerator4"))
        (set `self.FinaleUpdate` "NewEnumerator3")
        (else
          (set `self.Direction` (make `/Game/Players/Struct_Enum/STR_Direction2D` "NewEnumerator4" "NewEnumerator4"))
          (set `self.FinaleUpdate` "NewEnumerator0"))))))

(fn `UpdatePosition`
  (locals (PushX :type "Float (double-precision)") (PushY :type "Float (double-precision)"))
  (bind _springarm (`self.SpringArm`))
  (bind (_direction_x _direction_y) (break `/Game/Players/Struct_Enum/STR_Direction2D` (`self.Direction`)))
  (bind _rootcomponent (`self.RootComponent`))
  (bind _returnvalue (+ (`SpringArmComponent.TargetArmLength` (`self.SpringArm`)) 5.0))
  (bind _returnvalue_2 (+ (`SpringArmComponent.TargetArmLength` _springarm) -5.0))
  (switch `/Game/Players/Struct_Enum/EN_CamPattern` (`self.FinaleUpdate`)
    (:`NewEnumerator0`
      (if (> _returnvalue_2 (`self.ZommMin`))
        (bind _output_get (set `SpringArmComponent.TargetArmLength` _returnvalue_2 _springarm))))
    (:`NewEnumerator1`
      (if (< _returnvalue (`self.ZoomMax`))
        (set `SpringArmComponent.TargetArmLength` _returnvalue _springarm)))
    (:`NewEnumerator2`
      (`|ExecutionSequence`
        (:`then_0`
          (switch `/Game/Players/Struct_Enum/EN_Push` _direction_x
            (:`NewEnumerator2`
              (set `local.PushX` -12.0)
              (`SceneComponent.K2_SetWorldLocation` _rootcomponent (+ (`SceneComponent.K2_GetComponentLocation` _rootcomponent) (`KismetMathLibrary.MakeVector` 0.0 (`local.PushX`) (`local.PushY`))) false false :!label _label))
            (:`NewEnumerator3`
              (set `local.PushX` 12.0)
              (goto _label))
            (:`NewEnumerator4`
              (`KismetSystemLibrary.PrintText` "ERROR: DIRECTION SET OT NONE" true false (struct :`R` 1.0 :`B` 0.009101 :`A` 1.0) :!label _label_2))))
        (:`then_1`
          (switch `/Game/Players/Struct_Enum/EN_Push` _direction_y
            (:`NewEnumerator0`
              (set `local.PushY` 12.0)
              (goto _label))
            (:`NewEnumerator1`
              (set `local.PushY` -12.0)
              (goto _label))
            (:`NewEnumerator4`
              (goto _label_2))))))))

(fn `UserConstructionScript`)