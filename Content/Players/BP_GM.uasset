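; BP_GM is a game manager that spawns an extra local player and handles the end screen, restart and quit.
; BeginPlay creates the player, then caches and prints the count of all BP_PlayerBase actors.
; ShowEnd pauses the game and opens a lazily created, reused WBP_End with UI-only input and a visible cursor.
; Restart fires the OnRestart dispatcher, restores game input, unpauses and closes the widget.
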(event `self.ReceiveBeginPlay`
  (`GameplayStatics.CreatePlayer` -1)
  (bind _outactors (`GameplayStatics.GetAllActorsOfClass` "/Game/Players/BP_PlayerBase.BP_PlayerBase_C"))
  (set `self.Players` _outactors)
  (`KismetSystemLibrary.PrintString` (`KismetStringLibrary.Conv_IntToString` (`KismetArrayLibrary.Array_Length` _outactors))))

(fn `Quit`
  (`KismetSystemLibrary.QuitGame` null "Quit"))

(fn `Restart`
  (bind _returnvalue (`GameplayStatics.GetPlayerController` 0))
  (`self.OnRestart`)
  (`WidgetBlueprintLibrary.SetInputMode_GameOnly` _returnvalue)
  (set `PlayerController.bShowMouseCursor` false _returnvalue)
  (`GameplayStatics.SetGamePaused` false)
  (bind _endwidget (`self.EndWidget`)
    (:`then`
      (`/Game/Widgets/End/WBP_End.Close` _endwidget))
    (:`else`)))

(fn `ShowEnd`
  (bind _returnvalue (`GameplayStatics.GetPlayerController` 0))
  (`GameplayStatics.SetGamePaused` true)
  (bind _endwidget (`self.EndWidget`)
    (:`then`
      (`/Game/Widgets/End/WBP_End.Open` _endwidget))
    (:`else`
      (bind _returnvalue_2 (`|CreateWidget` "/Game/Widgets/End/WBP_End.WBP_End_C" (`GameplayStatics.GetPlayerController` 0)))
      (bind _output_get (set `self.EndWidget` _returnvalue_2))
      (`UserWidget.AddToViewport` _output_get 0)))
  (`WidgetBlueprintLibrary.SetInputMode_UIOnlyEx` _returnvalue _output_get)
  (set `PlayerController.bShowMouseCursor` true _returnvalue))

(fn `UserConstructionScript`)