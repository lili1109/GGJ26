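; Base player character for a two-sided red/blue game, with movement on a fixed plane, jumping and interaction with overlapping BP_BaseGPE actors.
; On possession it adds input mapping and picks BLUE for the first player controller, RED for others.
; SetSide swaps mask, material, Niagara ring and capsule channels, so each side ignores the other's channel.
; Game mode restarts reposition it near its player start, keeping X and randomizing Y.
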(event `self.ReceiveBeginPlay`
  (add `/Game/Players/BP_GM.OnRestart` (`self.GetGameMode`) (delegate `OnRestart_Event`)))

(event `OnRestart_Event`
  (`self.Restart`))

(event `self.ReceivePossessed`
  (params (NewController :type "Controller Object Reference"))
  (bind _asbp_controller (cast `/Game/Players/BP_Controller` NewController))
  (`EnhancedInputSubsystemInterface.AddMappingContext` (pcsubsystem `EnhancedInputLocalPlayerSubsystem` _asbp_controller) "/Game/Players/Input/IMC_Default.IMC_Default" 0 (struct))
  (if (!= _asbp_controller (`GameplayStatics.GetPlayerController` 0))
    (`self.SetSide` "NewEnumerator1")
    (else
      (`self.SetSide` "NewEnumerator0"))))

(event `EnhancedInput|/Game/Players/Input/InputAction/IA_Move`
  (params (ActionValue :type "Float (double-precision)") (ElapsedSeconds :type "Float (double-precision)") (TriggeredSeconds :type "Float (double-precision)") (InputAction :type "InputAction Object Reference" :default "/Game/Players/Input/InputAction/IA_Move.IA_Move"))
  (bind (_returnvalue_x _returnvalue_y _returnvalue_z) (`KismetMathLibrary.BreakVector` (`KismetMathLibrary.GetForwardVector` (`SceneComponent.RelativeRotation` (`self.Mesh`)))))
  (:`Triggered`
    (`self.AddMovementInput` (`KismetMathLibrary.MakeVector` 0.0 (* _returnvalue_y -1.0) _returnvalue_z) ActionValue)))

(event `EnhancedInput|/Game/Players/Input/InputAction/IA_Jump`
  (params (ActionValue :type Boolean) (ElapsedSeconds :type "Float (double-precision)") (TriggeredSeconds :type "Float (double-precision)") (InputAction :type "InputAction Object Reference" :default "/Game/Players/Input/InputAction/IA_Jump.IA_Jump"))
  (:`Started`
    (`self.Jump`)
    (set `self.IsJumping` true)))

(event `EnhancedInput|/Game/Players/Input/InputAction/IA_Interact`
  (params (ActionValue :type Boolean) (ElapsedSeconds :type "Float (double-precision)") (TriggeredSeconds :type "Float (double-precision)") (InputAction :type "InputAction Object Reference" :default "/Game/Players/Input/InputAction/IA_Interact.IA_Interact"))
  (:`Started`
    (for _array_element (`PrimitiveComponent.GetOverlappingActors` (`self.CapsuleComponent`) "/Game/Blueprints/GPE/BP_BaseGPE.BP_BaseGPE_C")
      (message `/Game/Blueprints/Interface/BPI_Interactable.StartInteraction` _array_element self)))
  (:`Completed`
    (for _array_element_2 (`PrimitiveComponent.GetOverlappingActors` (`self.CapsuleComponent`) "/Game/Blueprints/GPE/BP_BaseGPE.BP_BaseGPE_C")
      (message `/Game/Blueprints/Interface/BPI_Interactable.EndInteraction` _array_element_2 self))))

(event `self.ReceiveTick`
  (params (DeltaSeconds :type "Float (single-precision)"))
  (if (not (`NavMovementInterface.IsFalling` (`self.CharacterMovement`)))
    (set `self.IsJumping` false)))

(event `Key|R`
  (params (Key :type "Key Structure")))

(fn `GetGameMode`
  (returns (GameMode :type "/Game/Players/BP_GM Object Reference"))
  (`self.GameMode`
    (:`then`
      _)
    (:`else`
      (bind _asbp_gm (cast `/Game/Players/BP_GM` (`GameplayStatics.GetGameMode`)))
      (set `self.GameMode` _asbp_gm)))
  (return (`self.GameMode`)))

(fn `GetMask`
  (returns (Mask :type "/Game/Blueprints/MaskComponent/BP_Mask Object Reference"))
  (`self.Mask`
    (:`then`
      _)
    (:`else`
      (bind _asbp_mask (cast `/Game/Blueprints/MaskComponent/BP_Mask` (`ChildActorComponent.ChildActor` (`self.MaskComponent`))))
      (set `self.Mask` _asbp_mask)))
  (return (`self.Mask`)))

(fn `Restart`
  (bind _returnvalue_x (`KismetMathLibrary.BreakVector` (`self.K2_GetActorLocation`)))
  (bind (_returnvalue_x_2 _returnvalue_y _returnvalue_z) (`KismetMathLibrary.BreakVector` (`self.K2_GetActorLocation` (`GameModeBase.K2_FindPlayerStart` (`self.GetGameMode`) (`self.GetController`) ""))))
  (`self.K2_SetActorLocation` (`KismetMathLibrary.RandomPointInBoundingBox` (`KismetMathLibrary.MakeVector` _returnvalue_x _returnvalue_y _returnvalue_z) (0.0 50.0 0.0))))

(fn `SetSide`
  (params (Type :type "/Game/Blueprints/MaskComponent/E_Mask_Type Enum" :default "NewEnumerator0"))
  (switch `/Game/Blueprints/MaskComponent/E_Mask_Type` Type
    (:`NewEnumerator0`
      (set `/Game/Blueprints/MaskComponent/BP_Mask.Type` "NewEnumerator0" (`self.GetMask`))
      (`/Game/Blueprints/MaskComponent/BP_Mask.UpdateMaterial` (`self.GetMask`))
      (`PrimitiveComponent.SetCollisionObjectType` (`self.CapsuleComponent`) "ECC_GameTraceChannel1")
      (`PrimitiveComponent.SetCollisionResponseToChannel` (`self.CapsuleComponent`) "ECC_GameTraceChannel2" "ECR_Ignore")
      (`PrimitiveComponent.SetCollisionResponseToChannel` (`self.CapsuleComponent`) "ECC_GameTraceChannel1" "ECR_Block")
      (`PrimitiveComponent.SetMaterial` (`self.Mesh`) 1 "/Game/Material/M_blueE.M_blueE")
      (`NiagaraComponent.SetAsset` (`self.Niagara`) "/Game/Art/Niagara/NS_Ring_Blue.NS_Ring_Blue" true))
    (:`NewEnumerator1`
      (set `/Game/Blueprints/MaskComponent/BP_Mask.Type` "NewEnumerator1" (`self.GetMask`))
      (`/Game/Blueprints/MaskComponent/BP_Mask.UpdateMaterial` (`self.GetMask`))
      (`PrimitiveComponent.SetCollisionObjectType` (`self.CapsuleComponent`) "ECC_GameTraceChannel2")
      (`PrimitiveComponent.SetCollisionResponseToChannel` (`self.CapsuleComponent`) "ECC_GameTraceChannel1" "ECR_Ignore")
      (`PrimitiveComponent.SetCollisionResponseToChannel` (`self.CapsuleComponent`) "ECC_GameTraceChannel2" "ECR_Block")
      (`PrimitiveComponent.SetMaterial` (`self.Mesh`) 1 "/Game/Material/M_redE.M_redE")
      (`NiagaraComponent.SetAsset` (`self.Niagara`) "/Game/Art/Niagara/NS_Ring_Red.NS_Ring_Red" true))))

(fn `UserConstructionScript`)