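; BP_SimpleCam is a shared camera that frames two players and becomes the view target of player controller 0 on BeginPlay.
; Each tick it moves to the midpoint of the first two players in BP_GM's Players array.
; Spring arm length lerps between zoom limits by player distance over DistMax, unclamped, with camera lag enabled for smoothing.
; Step-based ZoomIn and ZoomOut functions exist but are not called here.
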(event `self.ReceiveBeginPlay`
  (`PlayerController.SetViewTargetWithBlend` (`GameplayStatics.GetPlayerController` 0) self 0.0 "VTBlend_Linear" 0.0 false)
  (bind _asbp_gm (cast `/Game/Players/BP_GM` (`GameplayStatics.GetGameMode`)))
  (set `self.GameMode` _asbp_gm)
  (set `SpringArmComponent.bEnableCameraLag` true (`self.SpringArm`)))

(event `self.ReceiveTick`
  (params (DeltaSeconds :type "Float (single-precision)"))
  (`self.GetData`)
  (`SceneComponent.K2_SetWorldLocation` (`self.DefaultSceneRoot`) (`self.CamPos`) false false))

(fn `GetData`
  (set `self.Player1World` (`self.K2_GetActorLocation` (`|GetArrayItem` (`/Game/Players/BP_GM.Players` (`self.GameMode`)))))
  (set `self.Player2World` (`self.K2_GetActorLocation` (`|GetArrayItem` (`/Game/Players/BP_GM.Players` (`self.GameMode`)) 1)))
  (set `self.CamPos` (`KismetMathLibrary.VLerp` (`self.Player1World`) (`self.Player2World`) 0.5))
  (bind _output_get (set `self.DistBetweenPlayers` (`KismetMathLibrary.Vector_Distance` (`self.Player1World`) (`self.Player2World`))))
  (`self.ZoomChange` (`KismetMathLibrary.Lerp` (`self.ZoomMin`) (`self.ZoomMax`) (/ _output_get (`self.DistMax`)))))

(fn `UserConstructionScript`)

(fn `ZoomChange`
  (params (Val :type "Float (double-precision)"))
  (set `SpringArmComponent.TargetArmLength` Val (`self.SpringArm`)))

(fn `ZoomIn`
  (params (Delta :type "Float (double-precision)"))
  (bind _springarm (`self.SpringArm`))
  (bind _returnvalue (+ (`SpringArmComponent.TargetArmLength` _springarm) (`self.Zoom-`)))
  (if (> _returnvalue (`self.ZoomMin`))
    (set `SpringArmComponent.TargetArmLength` _returnvalue _springarm)))

(fn `ZoomOut`
  (params (deltaTime :type "Float (double-precision)"))
  (bind _springarm (`self.SpringArm`))
  (bind _returnvalue (+ (`SpringArmComponent.TargetArmLength` _springarm) (`self.Zoom+`)))
  (if (< _returnvalue (`self.ZoomMax`))
    (set `SpringArmComponent.TargetArmLength` _returnvalue _springarm)))