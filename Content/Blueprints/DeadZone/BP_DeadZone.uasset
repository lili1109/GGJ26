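; BP_DeadZone is a trigger volume that restarts the game when the player enters it.
; Its Box overlap event checks that the other actor's class is exactly BP_PlayerBase, then calls Restart on the game mode.
; GetGm lazily casts the current game mode to BP_GM and caches it in GameMode for reuse.
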(event `self.Box.OnComponentBeginOverlap`
  (params (OverlappedComponent :type "PrimitiveComponent Object Reference") (OtherActor :type "Actor Object Reference") (OtherComp :type "PrimitiveComponent Object Reference") (OtherBodyIndex :type Integer) (bFromSweep :type Boolean) (SweepResult :type "HitResult Structure (by ref)"))
  (if (== (`GameplayStatics.GetObjectClass` OtherActor) "/Game/Players/BP_PlayerBase.BP_PlayerBase_C")
    (`/Game/Players/BP_GM.Restart` (`self.GetGm`))))

(fn `GetGm`
  (returns (GM :type "/Game/Players/BP_GM Object Reference"))
  (`self.GameMode`
    (:`then`
      _)
    (:`else`
      (bind _asbp_gm (cast `/Game/Players/BP_GM` (`GameplayStatics.GetGameMode`)))
      (set `self.GameMode` _asbp_gm)))
  (return (`self.GameMode`)))

(fn `UserConstructionScript`)