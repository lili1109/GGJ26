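; Hold-style gameplay button that relays start and end interaction to a linked InteractableGPE for players wearing the right mask.
; The interact box toggles an input prompt widget for matching players and sends an end message when one leaves.
; BeginPlay sets the prompt's key and type for blue or red buttons.
; The construction script sets mesh material parameters to show the base, all, blue or red variant.
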(event `self.ReceiveBeginPlay`
  (bind _wbp_input (`self.GetWidgetInput`))
  (bind _wbp_input_2 (`self.GetWidgetInput`))
  (bind _inputkey (`self.inputKey`))
  (`parent.ReceiveBeginPlay`)
  (switch `/Game/Blueprints/GPE/Enum_GPE_Type` (`self.Type`)
    (:`NewEnumerator2`
      (set `/Game/Widgets/Input/WBP_Input.KeyText` (`BlueprintMapLibrary.Map_Find` _inputkey "NewEnumerator0") _wbp_input_2)
      (set `/Game/Widgets/Input/WBP_Input.inputType` "NewEnumerator0" _wbp_input))
    (:`NewEnumerator3`
      (set `/Game/Widgets/Input/WBP_Input.KeyText` (`BlueprintMapLibrary.Map_Find` _inputkey "NewEnumerator1") _wbp_input_2)
      (set `/Game/Widgets/Input/WBP_Input.inputType` "NewEnumerator1" _wbp_input))))

(event `/Game/Blueprints/Interface/BPI_Interactable.StartInteraction`
  (params (Player :type "/Game/Players/BP_PlayerBase Object Reference"))
  (if (`self.IsRightMask` (`/Game/Players/BP_PlayerBase.GetMask` Player))
    (bind _interactablegpe (`self.InteractableGPE`)
      (:`then`
        (message `/Game/Blueprints/Interface/BPI_Interactable.StartInteraction` _interactablegpe Player))
      (:`else`))))

(event `/Game/Blueprints/Interface/BPI_Interactable.EndInteraction`
  (params (player :type "/Game/Players/BP_PlayerBase Object Reference"))
  (if (`self.IsRightMask` (`/Game/Players/BP_PlayerBase.GetMask` player))
    (bind _interactablegpe (`self.InteractableGPE`)
      (:`then`
        (message `/Game/Blueprints/Interface/BPI_Interactable.EndInteraction` _interactablegpe player))
      (:`else`))))

(event `self.InteractBox.OnComponentEndOverlap`
  (params (OverlappedComponent :type "PrimitiveComponent Object Reference") (OtherActor :type "Actor Object Reference") (OtherComp :type "PrimitiveComponent Object Reference") (OtherBodyIndex :type Integer))
  (if (not (`KismetArrayLibrary.Array_Contains` (`PrimitiveComponent.GetOverlappingActors` (`self.InteractBox`) "/Game/Players/BP_PlayerBase.BP_PlayerBase_C") OtherActor))
    (bind _asbp_player_base (cast `/Game/Players/BP_PlayerBase` OtherActor))
    (if (`self.IsRightMask` (`/Game/Players/BP_PlayerBase.GetMask` _asbp_player_base))
      (`SceneComponent.SetHiddenInGame` (`self.Widget`) true false)
      (bind _interactablegpe (`self.InteractableGPE`)
        (:`then`
          (message `/Game/Blueprints/Interface/BPI_Interactable.EndInteraction` _interactablegpe _asbp_player_base))
        (:`else`)))))

(event `self.InteractBox.OnComponentBeginOverlap`
  (params (OverlappedComponent :type "PrimitiveComponent Object Reference") (OtherActor :type "Actor Object Reference") (OtherComp :type "PrimitiveComponent Object Reference") (OtherBodyIndex :type Integer) (bFromSweep :type Boolean) (SweepResult :type "HitResult Structure (by ref)"))
  (bind _asbp_player_base (cast `/Game/Players/BP_PlayerBase` OtherActor))
  (if (`self.IsRightMask` (`/Game/Players/BP_PlayerBase.GetMask` _asbp_player_base))
    (`SceneComponent.SetHiddenInGame` (`self.Widget`) false false)))

(fn `GetWidgetInput`
  (returns (`WBP Input` :type "/Game/Widgets/Input/WBP_Input Object Reference"))
  (`self.WBP Input`
    (:`then`
      _)
    (:`else`
      (bind _aswbp_input (cast `/Game/Widgets/Input/WBP_Input` (`WidgetComponent.GetWidget` (`self.Widget`))))
      (set `self.WBP Input` _aswbp_input)))
  (return (`self.WBP Input`)))

(fn `UserConstructionScript`
  (`parent.UserConstructionScript`)
  (switch `/Game/Blueprints/GPE/Enum_GPE_Type` (`self.Type`)
    (:`NewEnumerator0`
      (`MeshComponent.SetScalarParameterValueOnMaterials` (`self.StaticMeshBlue1`) "IsBase" 1.0)
      (`MeshComponent.SetScalarParameterValueOnMaterials` (`self.StaticMeshBlue2`) "IsBase" 1.0)
      (`MeshComponent.SetScalarParameterValueOnMaterials` (`self.StaticMeshRed4`) "IsBase" 0.0)
      (`MeshComponent.SetScalarParameterValueOnMaterials` (`self.StaticMeshRed3`) "IsBase" 0.0)
      (`MeshComponent.SetScalarParameterValueOnMaterials` (`self.StaticMeshBlue1`) "IsAll" 1.0)
      (`MeshComponent.SetScalarParameterValueOnMaterials` (`self.StaticMeshBlue2`) "IsAll" 1.0)
      (`MeshComponent.SetScalarParameterValueOnMaterials` (`self.StaticMeshRed4`) "IsAll" 1.0)
      (`MeshComponent.SetScalarParameterValueOnMaterials` (`self.StaticMeshRed3`) "IsAll" 1.0))
    (:`NewEnumerator1`
      (`MeshComponent.SetScalarParameterValueOnMaterials` (`self.StaticMeshBlue1`) "IsAll" 1.0)
      (`MeshComponent.SetScalarParameterValueOnMaterials` (`self.StaticMeshBlue2`) "IsAll" 1.0)
      (`MeshComponent.SetScalarParameterValueOnMaterials` (`self.StaticMeshRed3`) "IsAll" 1.0)
      (`MeshComponent.SetScalarParameterValueOnMaterials` (`self.StaticMeshRed4`) "IsAll" 1.0)
      (`MeshComponent.SetScalarParameterValueOnMaterials` (`self.StaticMeshBlue1`) "Type" 0.0)
      (`MeshComponent.SetScalarParameterValueOnMaterials` (`self.StaticMeshBlue2`) "Type" 0.0)
      (`MeshComponent.SetScalarParameterValueOnMaterials` (`self.StaticMeshRed3`) "Type" 1.0)
      (`MeshComponent.SetScalarParameterValueOnMaterials` (`self.StaticMeshRed4`) "Type" 1.0)
      (`MeshComponent.SetScalarParameterValueOnMaterials` (`self.StaticMeshBlue1`) "IsBase" 0.0 :!label _label)
      (`MeshComponent.SetScalarParameterValueOnMaterials` (`self.StaticMeshBlue2`) "IsBase" 0.0)
      (`MeshComponent.SetScalarParameterValueOnMaterials` (`self.StaticMeshRed4`) "IsBase" 0.0)
      (`MeshComponent.SetScalarParameterValueOnMaterials` (`self.StaticMeshRed3`) "IsBase" 0.0))
    (:`NewEnumerator2`
      (`MeshComponent.SetScalarParameterValueOnMaterials` (`self.StaticMeshBlue1`) "Type" 0.0)
      (`MeshComponent.SetScalarParameterValueOnMaterials` (`self.StaticMeshBlue2`) "Type" 0.0)
      (`MeshComponent.SetScalarParameterValueOnMaterials` (`self.StaticMeshRed3`) "Type" 0.0)
      (`MeshComponent.SetScalarParameterValueOnMaterials` (`self.StaticMeshRed4`) "Type" 0.0)
      (`MeshComponent.SetScalarParameterValueOnMaterials` (`self.StaticMeshBlue1`) "IsAll" 0.0 :!label _label_2)
      (`MeshComponent.SetScalarParameterValueOnMaterials` (`self.StaticMeshBlue2`) "IsAll" 0.0)
      (`MeshComponent.SetScalarParameterValueOnMaterials` (`self.StaticMeshRed3`) "IsAll" 0.0)
      (`MeshComponent.SetScalarParameterValueOnMaterials` (`self.StaticMeshRed4`) "IsAll" 0.0)
      (goto _label))
    (:`NewEnumerator3`
      (`MeshComponent.SetScalarParameterValueOnMaterials` (`self.StaticMeshBlue1`) "Type" 1.0)
      (`MeshComponent.SetScalarParameterValueOnMaterials` (`self.StaticMeshBlue2`) "Type" 1.0)
      (`MeshComponent.SetScalarParameterValueOnMaterials` (`self.StaticMeshRed3`) "Type" 1.0)
      (`MeshComponent.SetScalarParameterValueOnMaterials` (`self.StaticMeshRed4`) "Type" 1.0)
      (goto _label_2))))