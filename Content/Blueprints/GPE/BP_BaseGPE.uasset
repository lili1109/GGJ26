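; Base gameplay element with a BASE, ALL, BLUE or RED type that switches collision channel when masks are added or removed.
; While a matching mask applies, Tick moves and resizes BlueBox and RedBox along Y from closest points on that mask's box.
; Player overlaps toggle that resizing, pausing it once the type's player requirement is met.
; It registers an empty Restart hook with BP_GM; construction ignores Type, leaving its material switch unwired.
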(event `self.ReceiveBeginPlay`
  (`self.InitCollision`)
  (add `/Game/Players/BP_GM.OnRestart` (`self.GetGameMode`) (delegate `OnRestart_Event`)))

(event `OnRestart_Event`
  (`self.Restart`))

(event `self.ReceiveTick`
  (params (DeltaSeconds :type "Float (single-precision)"))
  (if (`self.NeedUpdateCollisionsSize`)
    (`self.UpdateBoxCollision`)))

(event `self.OvelappBox.OnComponentBeginOverlap`
  (params (OverlappedComponent :type "PrimitiveComponent Object Reference") (OtherActor :type "Actor Object Reference") (OtherComp :type "PrimitiveComponent Object Reference") (OtherBodyIndex :type Integer) (bFromSweep :type Boolean) (SweepResult :type "HitResult Structure (by ref)"))
  (bind _asbp_player_base (cast `/Game/Players/BP_PlayerBase` OtherActor))
  (`KismetArrayLibrary.Array_AddUnique` (`self.Players`) _asbp_player_base)
  (if (`self.HasEnoughPlayers`)
    (`self.OnHasEnoughPlayerOverlap` true)))

(event `self.OvelappBox.OnComponentEndOverlap`
  (params (OverlappedComponent :type "PrimitiveComponent Object Reference") (OtherActor :type "Actor Object Reference") (OtherComp :type "PrimitiveComponent Object Reference") (OtherBodyIndex :type Integer))
  (if (not (`KismetArrayLibrary.Array_Contains` (`PrimitiveComponent.GetOverlappingActors` (`self.OvelappBox`) "/Game/Players/BP_PlayerBase.BP_PlayerBase_C") OtherActor))
    (bind _asbp_player_base (cast `/Game/Players/BP_PlayerBase` OtherActor))
    (`KismetArrayLibrary.Array_RemoveItem` (`self.Players`) _asbp_player_base)
    (if (not (`self.HasEnoughPlayers`))
      (`self.OnHasEnoughPlayerOverlap` false))))

(fn `AddMask`
  (params (NewMask :type "/Game/Blueprints/MaskComponent/BP_Mask Object Reference"))
  (`KismetArrayLibrary.Array_AddUnique` (`self.Masks`) NewMask)
  (`self.UpdateCollisionType`))

(fn `EnumMaskTypeToGPEType`
  (params (maskType :type "/Game/Blueprints/MaskComponent/E_Mask_Type Enum" :default "NewEnumerator0"))
  (returns (GPEType :type "/Game/Blueprints/GPE/Enum_GPE_Type Enum"))
  (switch `/Game/Blueprints/MaskComponent/E_Mask_Type` maskType
    (:`NewEnumerator0`
      (return "NewEnumerator2"))
    (:`NewEnumerator1`
      (return "NewEnumerator3"))))

(fn `GetGameMode`
  (returns (GameMode :type "/Game/Players/BP_GM Object Reference"))
  (`self.GameMode`
    (:`then`
      _)
    (:`else`
      (bind _asbp_gm (cast `/Game/Players/BP_GM` (`GameplayStatics.GetGameMode`)))
      (set `self.GameMode` _asbp_gm)))
  (return (`self.GameMode`)))

(fn `HasEnoughPlayers`
  (returns (hasEnought :type Boolean))
  (locals (RigthMask :type Boolean :default false))
  (switch `/Game/Blueprints/GPE/Enum_GPE_Type` (`self.Type`)
    (:`NewEnumerator0`
      (return true))
    (:`NewEnumerator1`
      (return (== (`KismetArrayLibrary.Array_Length` (`self.Players`)) 2)))
    (:`NewEnumerator2`
      _)
    (:`NewEnumerator3`
      _))
  (for _array_element (`self.Players`)
    (if (`self.IsRightMask` (`/Game/Players/BP_PlayerBase.GetMask` _array_element))
      (set `local.RigthMask` true)))
  (return (`local.RigthMask`)))

(fn `InitCollision`
  (switch `/Game/Blueprints/GPE/Enum_GPE_Type` (`self.Type`)
    (:`NewEnumerator0`
      (`self.SetCollisionObjectType` "ECC_GameTraceChannel3" :!label _label))
    (:`NewEnumerator1`
      (goto _label))
    (:`NewEnumerator2`
      (`self.SetCollisionObjectType` "ECC_GameTraceChannel1"))
    (:`NewEnumerator3`
      (`self.SetCollisionObjectType` "ECC_GameTraceChannel2"))))

(fn `IsRightMask`
  (params (Mask :type "/Game/Blueprints/MaskComponent/BP_Mask Object Reference"))
  (returns (isRightMask :type Boolean))
  (return (or (`|EnumEquality` (`self.EnumMaskTypeToGPEType` (`/Game/Blueprints/MaskComponent/BP_Mask.Type` Mask)) (`self.Type`)) (`|EnumEquality` (`self.Type`) "NewEnumerator1"))))

(fn `OnHasEnoughPlayerOverlap`
  (params (hasEnoughtPlayers :type Boolean))
  (set `self.NeedUpdateCollisionsSize` (not hasEnoughtPlayers)))

(fn `RemoveMask`
  (params (MaskToRemove :type "/Game/Blueprints/MaskComponent/BP_Mask Object Reference"))
  (bind _returnvalue (`KismetArrayLibrary.Array_RemoveItem` (`self.Masks`) MaskToRemove))
  (if _returnvalue
    (`self.UpdateCollisionType`)))

(fn `Restart`)

(fn `SetCollisionObjectType`
  (params (Channel :type "ECollisionChannel Enum" :default "ECC_WorldStatic"))
  (if (`|EnumInequality` Channel (`self.CurrentChannel`))
    (set `self.CurrentChannel` (`local.Channel`))
    (`PrimitiveComponent.SetCollisionObjectType` (`self.BlueBox`) (`self.CurrentChannel`))
    (`PrimitiveComponent.SetCollisionObjectType` (`self.RedBox`) (`self.CurrentChannel`))
    (`KismetSystemLibrary.PrintString` (`|GetEnumeratorNameAsString` (`self.CurrentChannel`)))))

(fn `UpdateBoxCollision`
  (bind _bluebox (`self.BlueBox`))
  (bind (_returnvalue_x _returnvalue_y _returnvalue_z) (`KismetMathLibrary.BreakVector` (`SceneComponent.K2_GetComponentLocation` _bluebox)))
  (bind (_returnvalue_x_2 _returnvalue_y_2) (`KismetMathLibrary.BreakVector` (`SceneComponent.K2_GetComponentLocation` (`self.SecondPoint`))))
  (bind (_returnvalue_x_3 _returnvalue_y_3) (`KismetMathLibrary.BreakVector` (`SceneComponent.K2_GetComponentLocation` (`self.FirstPoint`))))
  (bind (_returnvalue_x_4 _returnvalue_y_4 _returnvalue_z_2) (`KismetMathLibrary.BreakVector` (`BoxComponent.GetScaledBoxExtent` (`self.OvelappBox`))))
  (bind _box (`/Game/Blueprints/MaskComponent/BP_Mask.Box` (`self.CurrentMask`)))
  (bind _outpointonbody (`PrimitiveComponent.GetClosestPointOnCollision` _box (`SceneComponent.K2_GetComponentLocation` (`self.FirstPoint`)) "None"))
  (bind _outpointonbody_2 (`PrimitiveComponent.GetClosestPointOnCollision` _box (`SceneComponent.K2_GetComponentLocation` (`self.SecondPoint`)) "None"))
  (bind (_returnvalue_x_5 _returnvalue_y_5) (`KismetMathLibrary.BreakVector` (`KismetMathLibrary.VLerp` _outpointonbody _outpointonbody_2 0.5)))
  (bind _returnvalue (`KismetMathLibrary.Lerp` 0.0 _returnvalue_y_4 (/ (- (.y _outpointonbody_2) (.y _outpointonbody)) (- _returnvalue_y_2 _returnvalue_y_3))))
  (`self.CurrentMask`
    (:`then`
      (`SceneComponent.K2_SetWorldLocation` _bluebox (`KismetMathLibrary.MakeVector` _returnvalue_x_5 _returnvalue_y_5 _returnvalue_z) false false)
      (`SceneComponent.K2_SetWorldLocation` (`self.RedBox`) (`KismetMathLibrary.MakeVector` _returnvalue_x_5 _returnvalue_y_5 _returnvalue_z) false false)
      (`BoxComponent.SetBoxExtent` (`self.BlueBox`) (`KismetMathLibrary.MakeVector` _returnvalue_x_4 _returnvalue _returnvalue_z_2) true)
      (`BoxComponent.SetBoxExtent` (`self.RedBox`) (`KismetMathLibrary.MakeVector` _returnvalue_x_4 _returnvalue _returnvalue_z_2) true))
    (:`else`)))

(fn `UpdateCollisionType`
  (locals (HasSameCollisionType :type Boolean))
  (if (`|EnumInequality` (`self.Type`) "NewEnumerator0")
    (if (`KismetArrayLibrary.Array_IsEmpty` (`self.Masks`))
      (`self.InitCollision`)
      (set `self.NeedUpdateCollisionsSize` false)
      (set `self.CurrentMask` null)
      (else
        (for _array_element (`self.Masks`)
          (if (`self.IsRightMask` _array_element)
            (set `self.CurrentMask` _array_element)
            (set `local.HasSameCollisionType` true)))
        (if (`local.HasSameCollisionType`)
          (`self.SetCollisionObjectType` "ECC_GameTraceChannel3")
          (set `self.NeedUpdateCollisionsSize` true)
          (else
            (`self.InitCollision`)
            (set `self.CurrentMask` null)))))
    (else
      (set `self.NeedUpdateCollisionsSize` false)
      (set `self.CurrentMask` null))))

(fn `UserConstructionScript`
  (`MeshComponent.SetScalarParameterValueOnMaterials` (`self.StaticMeshBlue`) "IsBase" 1.0)
  (`MeshComponent.SetScalarParameterValueOnMaterials` (`self.StaticMeshRed`) "IsBase" 0.0)
  (`MeshComponent.SetScalarParameterValueOnMaterials` (`self.StaticMeshBlue`) "IsAll" 1.0)
  (`MeshComponent.SetScalarParameterValueOnMaterials` (`self.StaticMeshRed`) "IsAll" 1.0))