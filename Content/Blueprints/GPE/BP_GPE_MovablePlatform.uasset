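; A movable platform gameplay element that travels between two relative positions and responds to how many players overlap it.
; The construction script feeds both points to an InterpToMovement component, finalised on BeginPlay.
; Toggling the root's mobility between Movable and Static follows the player-count check, while Restart restores the initial location and restarts interpolation, leaving it Static.
; Blue and red box hit events print colored debug names.
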(event `self.ReceiveBeginPlay`
  (`parent.ReceiveBeginPlay`)
  (`InterpToMovementComponent.FinaliseControlPoints` (`self.InterpToMovement`))
  (set `self.InitLocation` (`self.K2_GetActorLocation`)))

(event `self.ReceiveTick`
  (params (DeltaSeconds :type "Float (single-precision)"))
  (`parent.ReceiveTick` DeltaSeconds))

(event `self.BlueBox.OnComponentHit`
  (params (HitComponent :type "PrimitiveComponent Object Reference") (OtherActor :type "Actor Object Reference") (OtherComp :type "PrimitiveComponent Object Reference") (NormalImpulse :type "Vector Structure") (Hit :type "HitResult Structure (by ref)"))
  (`KismetSystemLibrary.PrintString` (`KismetSystemLibrary.GetDisplayName` HitComponent) true true (struct :`G` 0.06327 :`B` 1.0 :`A` 1.0)))

(event `self.RedBox.OnComponentHit`
  (params (HitComponent :type "PrimitiveComponent Object Reference") (OtherActor :type "Actor Object Reference") (OtherComp :type "PrimitiveComponent Object Reference") (NormalImpulse :type "Vector Structure") (Hit :type "HitResult Structure (by ref)"))
  (`KismetSystemLibrary.PrintString` (`KismetSystemLibrary.GetDisplayName` HitComponent) true true (struct :`R` 1.0 :`G` 0.052334 :`A` 1.0)))

(fn `OnHasEnoughPlayerOverlap`
  (params (hasEnoughtPlayers :type Boolean))
  (`parent.OnHasEnoughPlayerOverlap` hasEnoughtPlayers)
  (if (`self.HasEnoughPlayers`)
    (`SceneComponent.SetMobility` (`self.DefaultSceneRoot`) "Movable")
    (else
      (`SceneComponent.SetMobility` (`self.DefaultSceneRoot`) "Static"))))

(fn `Restart`
  (`parent.Restart`)
  (`SceneComponent.SetMobility` (`self.DefaultSceneRoot`) "Movable")
  (`self.K2_SetActorLocation` (`self.InitLocation`))
  (`InterpToMovementComponent.RestartMovement` (`self.InterpToMovement`) 1.0)
  (`SceneComponent.SetMobility` (`self.DefaultSceneRoot`) "Static"))

(fn `UserConstructionScript`
  (`parent.UserConstructionScript`)
  (`InterpToMovementComponent.AddControlPointPosition` (`self.InterpToMovement`) (`self.FirstPos`) true)
  (`InterpToMovementComponent.AddControlPointPosition` (`self.InterpToMovement`) (`self.SecondPos`) true))