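; BP_GPE_Door is an interactable door that moves vertically when an interaction starts and returns when it ends.
; StartInteraction and EndInteraction call OpenDoor, which ignores repeated states and plays or reverses a Timeline.
; The Timeline's Z value offsets the whole actor from the location cached at BeginPlay, using a swept move on update and finish.
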(event `self.ReceiveBeginPlay`
  (`parent.ReceiveBeginPlay`)
  (set `self.StartPosititon` (`self.K2_GetActorLocation`)))

(event `/Game/Blueprints/Interface/BPI_Interactable.StartInteraction`
  (params (Player :type "/Game/Players/BP_PlayerBase Object Reference"))
  (`self.OpenDoor` true))

(event `OpenDoor`
  (params (isOpen :type Boolean))
  (bind (_startposititon_x _startposititon_y _startposititon_z) (`KismetMathLibrary.BreakVector` (`self.StartPosititon`)))
  (if (!= isOpen (`self.isOpen`))
    (bind _output_get (set `self.isOpen` (not (`self.isOpen`))))
    (if _output_get
      (bind (_direction _z) (`Timeline|Timeline` :!label _label)
        (:`Update`
          _)
        (:`Finished`
          _))
      (`self.K2_SetActorLocation` (`KismetMathLibrary.MakeVector` _startposititon_x _startposititon_y (+ _startposititon_z _z)) true)
      (else
        (goto _label :!via `Reverse`)))))

(event `/Game/Blueprints/Interface/BPI_Interactable.EndInteraction`
  (params (player :type "/Game/Players/BP_PlayerBase Object Reference"))
  (`self.OpenDoor` false))

(fn `UserConstructionScript`
  (`parent.UserConstructionScript`))